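; Structure Blueprint for buildings that repeatedly produce friendly worker units.
; Each Tick turns the interface widget toward the player's RaceControllerPawn_BP camera, billboard style.
; Tick also feeds a five-second Delay into SpawnUnit, so the latent node acts as a repeating timer because it ignores re-triggers while pending.
; BeginPlay and the construction script are empty.
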(event `self.ReceiveBeginPlay`)

(event `self.ReceiveTick`
  (params (DeltaSeconds :type "Float (single-precision)"))
  (bind _interfacewidget (`self.InterfaceWidget`))
  (`|ExecutionSequence`
    (:`then_0`
      (bind _asrace_controller_pawn_bp (cast `/Game/NonGenerated/Blueprints/RaceControllerPawn_BP` (`GameplayStatics.GetPlayerPawn` 0)))
      (`SceneComponent.K2_SetWorldRotation` _interfacewidget (`KismetMathLibrary.FindLookAtRotation` (`SceneComponent.K2_GetComponentLocation` _interfacewidget) (`SceneComponent.K2_GetComponentLocation` (`/Game/NonGenerated/Blueprints/RaceControllerPawn_BP.Camera` _asrace_controller_pawn_bp))) false false))
    (:`then_1`
      (`KismetSystemLibrary.Delay` 5.0)
      (`self.SpawnUnit` "/Game/NonGenerated/Blueprints/Units/WorkerUnit_BP.WorkerUnit_BP_C" "STP_Friendly"))))

(fn `UserConstructionScript`)