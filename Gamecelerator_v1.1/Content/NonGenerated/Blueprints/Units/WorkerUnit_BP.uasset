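; WorkerUnit_BP is a worker unit with a health bar and a gather collision sphere sized to twice its gather distance.
; Construction gives its mesh a dynamic material, which Tick recolors by the unit's status toward the local player when selected, or red otherwise.
; Tick also billboards the health bar toward the camera, and GetDamaged subtracts health and refreshes the bar widget cached at BeginPlay.
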(event `self.ReceiveBeginPlay`
  (`|ExecutionSequence`
    (:`then_0`
      (bind _ashealth_bar_widget (cast `/Game/NonGenerated/UI/Widget/HealthBarWidget` (`WidgetComponent.GetUserWidgetObject` (`self.HealthBar`))))
      (set `self.HealthBar Instance` _ashealth_bar_widget))))

(event `self.ReceiveTick`
  (params (DeltaSeconds :type "Float (single-precision)"))
  (bind _materialinstance (`self.MaterialInstance`))
  (`|ExecutionSequence`
    (:`then_0`
      (if (`self.isSelected`)
        (switch `EStatusToPlayer` (`self.GetStatusToPlayer` (`GameplayStatics.GetPlayerController` 0))
          (:`STP_Owned`
            (`MaterialInstanceDynamic.SetVectorParameterValue` _materialinstance "Param" (struct :`R` 0.348925 :`G` 0.984375 :`B` 0.301046 :`A` 1.0) :!label _label))
          (:`STP_Friendly`
            (goto _label))
          (:`STP_Neutral`
            (`MaterialInstanceDynamic.SetVectorParameterValue` _materialinstance "Param" (struct :`R` 0.984375 :`G` 0.848365 :`A` 1.0)))
          (:`STP_Hostile`
            (`MaterialInstanceDynamic.SetVectorParameterValue` _materialinstance "Param" (struct :`R` 0.984375 :`G` 0.18457 :`B` 0.195801 :`A` 1.0)))
          (:`STP_None`
            (`MaterialInstanceDynamic.SetVectorParameterValue` _materialinstance "Param" (struct :`R` 0.317708 :`G` 0.317708 :`B` 0.317708 :`A` 1.0))))
        (else
          (`MaterialInstanceDynamic.SetVectorParameterValue` (`self.MaterialInstance`) "Param" (struct :`R` 1.0 :`B` 0.032916 :`A` 1.0)))))
    (:`then_1`
      (`SceneComponent.K2_SetWorldRotation` (`self.HealthBar`) (`KismetMathLibrary.FindLookAtRotation` (`SceneComponent.K2_GetComponentLocation` (`self.HealthBar`)) (`PlayerCameraManager.GetCameraLocation` (`GameplayStatics.GetPlayerCameraManager` 0))) false false))))

(event `self.GetDamaged`
  (params (amount :type "Float (single-precision)"))
  (bind _returnvalue (`self.SetHealth` (- (`self.GetHealth`) amount)))
  (`/Game/NonGenerated/UI/Widget/HealthBarWidget.UpdateHealth` (`self.HealthBar Instance`) _returnvalue (`self.GetMaxHealth`)))

(fn `UserConstructionScript`
  (`|ExecutionSequence`
    (:`then_0`
      (bind _returnvalue (`KismetMaterialLibrary.CreateDynamicMaterialInstance` "/Game/NonGenerated/Materials/Red.Red"))
      (bind _output_get (set `self.MaterialInstance` _returnvalue))
      (`PrimitiveComponent.SetMaterial` (`self.StaticMesh`) 0 _output_get))
    (:`then_1`
      (`SphereComponent.SetSphereRadius` (`self.GatherCollision`) (* (`self.GatherDistance`) 2.0) true))))