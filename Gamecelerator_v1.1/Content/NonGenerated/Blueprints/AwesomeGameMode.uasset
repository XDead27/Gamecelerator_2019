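; Game mode that groups the level's controllers by team when play begins.
; On BeginPlay it scans all Controller actors for those with exactly one DiplomacyHandlerComponent, then uses that component's ParentControllerTeamIndex to add each to the Neutral, Team1 or Team2 array.
; A second sequence step loops over RaceControllers with an empty body, and the construction script is empty.
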(event `self.ReceiveBeginPlay`
  (`|ExecutionSequence`
    (:`then_0`
      (bind _outactors (`GameplayStatics.GetAllActorsOfClass` "/Script/Engine.Controller"))
      (for _array_element _outactors
        (bind _returnvalue (`self.K2_GetComponentsByClass` _array_element "/Script/Gamecelerator_v1.DiplomacyHandlerComponent"))
        (if (== (`KismetArrayLibrary.Array_Length` _returnvalue) 1)
          (bind _ascontroller (cast `Controller` _array_element))
          (for _array_element_2 _returnvalue
            (switch `int` (`DiplomacyHandlerComponent.ParentControllerTeamIndex` _array_element_2)
              (:`0`
                (`KismetArrayLibrary.Array_Add` (`self.Neutral`) _ascontroller))
              (:`1`
                (`KismetArrayLibrary.Array_Add` (`self.Team_1`) _ascontroller))
              (:`2`
                (`KismetArrayLibrary.Array_Add` (`self.Team_2`) _ascontroller)))))))
    (:`then_1`
      (for _ (`self.RaceControllers`)
        _))))

(fn `UserConstructionScript`)