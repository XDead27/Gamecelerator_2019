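; Structure Blueprint that produces worker units and carries a world-space interface widget.
; Each Tick turns the widget to face the camera of the player's spectator pawn.
; Tick also feeds a five-second Delay that calls SpawnUnit with WorkerUnit_BP, so workers spawn repeatedly on that interval without a separate timer.
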(event `self.ReceiveBeginPlay`)

(event `self.ReceiveTick`
  (params (DeltaSeconds :type "Float (single-precision)"))
  (bind _interfacewidget (`self.InterfaceWidget`))
  (`|ExecutionSequence`
    (:`then_0`
      (bind _asplayer_spectator_pawn (cast `/Game/NonGenerated/Blueprints/PlayerSpectatorPawn` (`GameplayStatics.GetPlayerPawn` 0)))
      (`SceneComponent.K2_SetWorldRotation` _interfacewidget (`KismetMathLibrary.FindLookAtRotation` (`SceneComponent.K2_GetComponentLocation` _interfacewidget) (`SceneComponent.K2_GetComponentLocation` (`/Game/NonGenerated/Blueprints/PlayerSpectatorPawn.Camera` _asplayer_spectator_pawn))) false false))
    (:`then_1`
      (`KismetSystemLibrary.Delay` 5.0)
      (`self.SpawnUnit` "/Game/NonGenerated/Blueprints/WorkerUnit_BP.WorkerUnit_BP_C"))))

(fn `UserConstructionScript`)